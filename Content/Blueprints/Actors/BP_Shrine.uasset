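; Shrine actor that shows a rotating weapon, health or speed pickup and grants it to the player who claims it.
; The first game character to overlap it while active becomes owner through a DoOnce, and only that owner can collect.
; Collection calls the player's events to deactivate the shrine, then after a delay reactivate it, and a random pickup refills the child actor.
; Status switches material and sound; the authority seeds the initial pickup.
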(event OnComponentBeginOverlap(Capsule)
  (params (OverlappedComponent :type Primitive%20Component%20Object%20Reference) (OtherActor :type Actor%20Object%20Reference) (OtherComp :type Primitive%20Component%20Object%20Reference) (OtherBodyIndex :type Integer) (bFromSweep :type Boolean) (SweepResult :type Hit%20Result%20Structure%20%28by%20ref%29))
  (if (Pawn|IsLocalController (Game|GetPlayerController 0))
    (if (Utilities|Enum|Equal(Enum) (Variables|Default|GetShrineStatus) "NewEnumerator0")
      (bind _aschar_game (Utilities|Casting|CastToChar_Game OtherActor))
      (Utilities|FlowControl|Sequence
        (:then_0
          (Utilities|FlowControl|DoOnce false
            (:Completed
              (bind _output_get (Variables|Default|SetOwningPlayer _aschar_game))
              (Default|OCShrinePossess _output_get))))
        (:then_1
          (if (== _aschar_game (Variables|Default|GetOwningPlayer))
            (Default|OCShrtineStatus (Variables|Default|GetOwningPlayer) self "NewEnumerator1")
            (Default|GetPickUp (Variables|Default|GetOwningPlayer) (Variables|Default|GetShrineType))
            (ChildActorComponent|SetChildActorClass (Variables|Default|GetChildActor) 0)
            (Utilities|FlowControl|Delay 22.0)
            (Default|OCShrtineStatus (Variables|Default|GetOwningPlayer) self "NewEnumerator0")
            (CallFunction|SAShrineRecharge (Math|Random|RandomIntegerinRange 0 5))))))))

(event Custom|SA_ShrineRecharge
  (params (Selection :type Integer))
  (CallFunction|ShrineRecharge Selection))

(event EventTick
  (params (DeltaSeconds :type Float%20%28single-precision%29))
  (if (Utilities|Enum|NotEqual(Enum) (Variables|Default|GetShrineStatus) "NewEnumerator1")
    (Transformation|AddRelativeRotation (Variables|Default|GetChildActor) "0,2.000000, 0" false false)))

(event EventBeginPlay
  (Networking|SwitchHasAuthority
    (:Authority
      (CallFunction|SAShrineRecharge))))

(fn ConstructionScript
  (CallFunction|SetShrineStatus (Variables|Default|GetShrineStatus)))

(fn SetShrineStatus
  (params (ShrineStatus :type E_ShrineStatus%20Enum :default "NewEnumerator0"))
  (bind _staticmesh (Variables|Default|GetStaticMesh))
  (switch Utilities|FlowControl|Switch|SwitchonE_ShrineStatus ShrineStatus
    (:NewEnumerator0
      (Rendering|Material|SetMaterial _staticmesh 0 "/Game/Materials/M_Shrine_Active.M_Shrine_Active")
      (Variables|Default|SetShrineStatus "NewEnumerator0")
      (Audio|PlaySoundatLocation "/Game/Sounds/impactMining_003.impactMining_003" (Transformation|GetActorLocation self) "0, 0, 0" 1.0 1.0 0.0 0 0 0))
    (:NewEnumerator1
      (Rendering|Material|SetMaterial _staticmesh 0 "/Game/Materials/M_Shrine_Inactive.M_Shrine_Inactive")
      (Variables|Default|SetShrineStatus "NewEnumerator1"))
    (:NewEnumerator2
      (Rendering|Material|SetMaterial _staticmesh 0 "/Game/Materials/M_Shrine_Locked.M_Shrine_Locked")
      (Variables|Default|SetShrineStatus "NewEnumerator2")
      (Audio|PlaySoundatLocation "/Game/Sounds/impactGlass_heavy_004.impactGlass_heavy_004" (Transformation|GetActorLocation self) "0, 0, 0" 1.0 1.0 0.0 0 0 0))))

(fn ShrineRecharge
  (params (Selection :type Integer))
  (bind _childactor (Variables|Default|GetChildActor))
  (switch int Selection
    (:0
      (ChildActorComponent|SetChildActorClass _childactor "/Game/Blueprints/Actors/PickUps/BP_PickUps_Weapons_01.BP_PickUps_Weapons_01_C")
      (Variables|Default|SetShrineType "NewEnumerator4"))
    (:1
      (ChildActorComponent|SetChildActorClass _childactor "/Game/Blueprints/Actors/PickUps/BP_PickUps_Weapons_02.BP_PickUps_Weapons_02_C")
      (Variables|Default|SetShrineType "NewEnumerator5"))
    (:2
      (ChildActorComponent|SetChildActorClass _childactor "/Game/Blueprints/Actors/PickUps/BP_PickUps_Weapons_03.BP_PickUps_Weapons_03_C")
      (Variables|Default|SetShrineType "NewEnumerator6"))
    (:3
      (ChildActorComponent|SetChildActorClass _childactor "/Game/Blueprints/Actors/PickUps/BP_PickUps_Weapons_04.BP_PickUps_Weapons_04_C")
      (Variables|Default|SetShrineType "NewEnumerator8"))
    (:4
      (ChildActorComponent|SetChildActorClass _childactor "/Game/Blueprints/Actors/PickUps/BP_Health.BP_Health_C")
      (Variables|Default|SetShrineType "NewEnumerator1"))
    (:5
      (ChildActorComponent|SetChildActorClass _childactor "/Game/Blueprints/Actors/PickUps/BP_Speed.BP_Speed_C")
      (Variables|Default|SetShrineType "NewEnumerator3"))))

(fn ResetShrine
  (CallFunction|SetShrineStatus "NewEnumerator0")
  (Variables|Default|SetOwningPlayer 0))