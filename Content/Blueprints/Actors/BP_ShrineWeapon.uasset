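; Networked weapon shrine that displays a spinning random weapon pickup and grants it to an overlapping player.
; The authority picks one of four weapons at BeginPlay, setting the child actor and shrine type.
; Overlap runs only for locally controlled characters, routing weapon grant, status changes and post-cooldown recharge through Char_Game calls.
; Active, Inactive and Locked states swap the mesh material, with sounds for Active and Locked.
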(event OnComponentBeginOverlap(Capsule)
  (params (OverlappedComponent :type Primitive%20Component%20Object%20Reference) (OtherActor :type Actor%20Object%20Reference) (OtherComp :type Primitive%20Component%20Object%20Reference) (OtherBodyIndex :type Integer) (bFromSweep :type Boolean) (SweepResult :type Hit%20Result%20Structure%20%28by%20ref%29))
  ;[1 1 1] OnOverlapp
  (bind _aschar_game (Utilities|Casting|CastToChar_Game OtherActor))
  (if (Pawn|IsLocallyControlled _aschar_game)
    (if (Utilities|Enum|Equal(Enum) (Variables|Default|GetShrineStatus) "NewEnumerator0")
      (Utilities|FlowControl|Sequence
        (:then_0
          (Utilities|FlowControl|DoOnce false
            (:Completed
              (bind _output_get (Variables|Default|SetOwningPlayer _aschar_game))
              (Default|OCShrinePossess _output_get))))
        (:then_1
          (if (== _aschar_game (Variables|Default|GetOwningPlayer))
            (Default|OCShrtineStatus (Variables|Default|GetOwningPlayer) self "NewEnumerator1")
            (Default|GeWeapon (Variables|Default|GetOwningPlayer) (Variables|Default|GetShrineType) self)
            (Utilities|FlowControl|Delay 22.0)
            (Utilities|IsValid (Variables|Default|GetOwningPlayer)
              (:Is%20Valid
                (Default|OCShrtineStatus (Variables|Default|GetOwningPlayer) self "NewEnumerator0")
                (Default|SShrineRecharge (Variables|Default|GetOwningPlayer) self)))))))))

(event Custom|SA_ShrineRecharge
  (params (Selection :type Integer))
  ;[1 1 1] BeginPlay, Shrine Recharge
  (CallFunction|ShrineRecharge Selection))

(event Custom|ResetShrine
  ;[1 1 1] OnOverlapp
  (CallFunction|SetShrineStatus "NewEnumerator0")
  (Variables|Default|SetOwningPlayer 0)
  (Utilities|FlowControl|DoOnce false) ; enters at Reset
)

(event EventTick
  (params (DeltaSeconds :type Float%20%28single-precision%29))
  (if (Utilities|Enum|NotEqual(Enum) (Variables|Default|GetShrineStatus) "NewEnumerator1")
    (Transformation|AddRelativeRotation (Variables|Default|GetChildActor) "0,2.000000, 0" false false)))

(event EventBeginPlay
  ;[1 1 1] BeginPlay, Shrine Recharge
  (Networking|SwitchHasAuthority
    (:Authority
      (CallFunction|SAShrineRecharge (Math|Random|RandomIntegerinRange 1 4)))))

(fn ConstructionScript
  (CallFunction|SetShrineStatus (Variables|Default|GetShrineStatus)))

(fn SetShrineStatus
  (params (ShrineStatus :type E_ShrineStatus%20Enum :default "NewEnumerator0"))
  (bind _staticmesh (Variables|Default|GetStaticMesh))
  (switch Utilities|FlowControl|Switch|SwitchonE_ShrineStatus ShrineStatus
    (:NewEnumerator0
      (Rendering|Material|SetMaterial _staticmesh 0 "/Game/Materials/M_Shrine_Active.M_Shrine_Active")
      (Variables|Default|SetShrineStatus "NewEnumerator0")
      (Audio|PlaySoundatLocation "/Game/Sounds/impactMining_003.impactMining_003" (Transformation|GetActorLocation self) "0, 0, 0" 1.0 1.0 0.0 0 0 0))
    (:NewEnumerator1
      (Rendering|Material|SetMaterial _staticmesh 0 "/Game/Materials/M_Shrine_Inactive.M_Shrine_Inactive")
      (Variables|Default|SetShrineStatus "NewEnumerator1"))
    (:NewEnumerator2
      (Rendering|Material|SetMaterial _staticmesh 0 "/Game/Materials/M_Shrine_Locked.M_Shrine_Locked")
      (Variables|Default|SetShrineStatus "NewEnumerator2")
      (Audio|PlaySoundatLocation "/Game/Sounds/impactGlass_heavy_004.impactGlass_heavy_004" (Transformation|GetActorLocation self) "0, 0, 0" 1.0 1.0 0.0 0 0 0))))

(fn ShrineRecharge
  (params (Selection :type Integer))
  (bind _childactor (Variables|Default|GetChildActor))
  (switch int Selection
    (:0
      (ChildActorComponent|SetChildActorClass _childactor 0)
      (Variables|Default|SetShrineType "NewEnumerator0"))
    (:1
      (ChildActorComponent|SetChildActorClass _childactor "/Game/Blueprints/Actors/PickUps/BP_PickUps_Weapons_01.BP_PickUps_Weapons_01_C")
      (Variables|Default|SetShrineType "NewEnumerator4"))
    (:2
      (ChildActorComponent|SetChildActorClass _childactor "/Game/Blueprints/Actors/PickUps/BP_PickUps_Weapons_02.BP_PickUps_Weapons_02_C")
      (Variables|Default|SetShrineType "NewEnumerator5"))
    (:3
      (ChildActorComponent|SetChildActorClass _childactor "/Game/Blueprints/Actors/PickUps/BP_PickUps_Weapons_03.BP_PickUps_Weapons_03_C")
      (Variables|Default|SetShrineType "NewEnumerator6"))
    (:4
      (ChildActorComponent|SetChildActorClass _childactor "/Game/Blueprints/Actors/PickUps/BP_PickUps_Weapons_04.BP_PickUps_Weapons_04_C")
      (Variables|Default|SetShrineType "NewEnumerator8"))))