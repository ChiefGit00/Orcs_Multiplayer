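; Ability shrine actor that grants an overlapping Char_Game an ability matching its randomly chosen type, displayed as a health or speed child actor.
; On authority, pickup disables the capsule, clears the display and sets the shrine inactive, then reactivates and rerolls after a delay.
; Status drives material and sound, and the child actor spins on Tick unless inactive.
; The recharge roll can reach 3, which ShrineRecharge does not handle.
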(event OnComponentBeginOverlap(Capsule)
  (params (OverlappedComponent :type Primitive%20Component%20Object%20Reference) (OtherActor :type Actor%20Object%20Reference) (OtherComp :type Primitive%20Component%20Object%20Reference) (OtherBodyIndex :type Integer) (bFromSweep :type Boolean) (SweepResult :type Hit%20Result%20Structure%20%28by%20ref%29))
  ;[1 1 1] OnOverlapp
  (Networking|SwitchHasAuthority
    (:Authority
      (bind _aschar_game (Utilities|Casting|CastToChar_Game OtherActor))
      (if (Utilities|Enum|Equal(Enum) (Variables|Default|GetShrineStatus) "NewEnumerator0")
        (Collision|SetCollisionEnabled (Variables|Default|GetCapsule) "NoCollision")
        (CallFunction|ASetShrineStatus "NewEnumerator1")
        (Default|GetAbility _aschar_game (Variables|Default|GetShrineType))
        (ChildActorComponent|SetChildActorClass (Variables|Default|GetChildActor) 0)
        (Utilities|FlowControl|Delay 15.0)
        (Collision|SetCollisionEnabled (Variables|Default|GetCapsule) "QueryAndPhysics")
        (CallFunction|ASetShrineStatus "NewEnumerator0")
        (CallFunction|SAShrineRecharge (Math|Random|RandomIntegerinRange 1 3))))))

(event Custom|SA_ShrineRecharge
  (params (Selection :type Integer))
  ;[1 1 1] BeginPlay, Shrine Recharge
  (CallFunction|ShrineRecharge Selection))

(event Custom|ResetShrine
  ;[1 1 1] OnOverlapp
  (CallFunction|SetShrineStatus "NewEnumerator0"))

(event Custom|A_SetShrineStatus
  (params (ShrineStatus :type E_ShrineStatus%20Enum :default "NewEnumerator0"))
  (CallFunction|SetShrineStatus ShrineStatus))

(event EventTick
  (params (DeltaSeconds :type Float%20%28single-precision%29))
  (if (Utilities|Enum|NotEqual(Enum) (Variables|Default|GetShrineStatus) "NewEnumerator1")
    (Transformation|AddRelativeRotation (Variables|Default|GetChildActor) "0,2.000000, 0" false false)))

(event EventBeginPlay
  ;[1 1 1] BeginPlay, Shrine Recharge
  (Networking|SwitchHasAuthority
    (:Authority
      (CallFunction|SAShrineRecharge (Math|Random|RandomIntegerinRange 1 2)))))

(fn ConstructionScript
  (CallFunction|SetShrineStatus (Variables|Default|GetShrineStatus)))

(fn SetShrineStatus
  (params (ShrineStatus :type E_ShrineStatus%20Enum :default "NewEnumerator0"))
  (bind _staticmesh (Variables|Default|GetStaticMesh))
  (switch Utilities|FlowControl|Switch|SwitchonE_ShrineStatus ShrineStatus
    (:NewEnumerator0
      (Rendering|Material|SetMaterial _staticmesh 0 "/Game/Materials/M_Shrine_Active.M_Shrine_Active")
      (Variables|Default|SetShrineStatus "NewEnumerator0")
      (Audio|PlaySoundatLocation "/Game/Sounds/impactMining_003.impactMining_003" (Transformation|GetActorLocation self) "0, 0, 0" 1.0 1.0 0.0 0 0 0))
    (:NewEnumerator1
      (Rendering|Material|SetMaterial _staticmesh 0 "/Game/Materials/M_Shrine_Inactive.M_Shrine_Inactive")
      (Variables|Default|SetShrineStatus "NewEnumerator1"))
    (:NewEnumerator2
      (Rendering|Material|SetMaterial _staticmesh 0 "/Game/Materials/M_Shrine_Locked.M_Shrine_Locked")
      (Variables|Default|SetShrineStatus "NewEnumerator2")
      (Audio|PlaySoundatLocation "/Game/Sounds/impactGlass_heavy_004.impactGlass_heavy_004" (Transformation|GetActorLocation self) "0, 0, 0" 1.0 1.0 0.0 0 0 0))))

(fn ShrineRecharge
  (params (Selection :type Integer))
  (bind _childactor (Variables|Default|GetChildActor))
  (switch int Selection
    (:0
      (ChildActorComponent|SetChildActorClass _childactor 0)
      (Variables|Default|SetShrineType "NewEnumerator0"))
    (:1
      (ChildActorComponent|SetChildActorClass _childactor "/Game/Blueprints/Actors/PickUps/BP_Health.BP_Health_C")
      (Variables|Default|SetShrineType "NewEnumerator1"))
    (:2
      (ChildActorComponent|SetChildActorClass _childactor "/Game/Blueprints/Actors/PickUps/BP_Speed.BP_Speed_C")
      (Variables|Default|SetShrineType "NewEnumerator3"))))