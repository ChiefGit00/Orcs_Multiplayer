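; Weapon pickup Blueprint that handles server-authoritative melee-style hit damage through an attack collision component.
; An overlap while the Attack flag is set damages any Char_Game other than the owning player after a one-second delay.
; The hit clears the flag and disables the collision first, then re-enables the collision one second after the damage, leaving the flag cleared.
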(event OnComponentBeginOverlap(Coll_Attack)
  (params (OverlappedComponent :type Primitive%20Component%20Object%20Reference) (OtherActor :type Actor%20Object%20Reference) (OtherComp :type Primitive%20Component%20Object%20Reference) (OtherBodyIndex :type Integer) (bFromSweep :type Boolean) (SweepResult :type Hit%20Result%20Structure%20%28by%20ref%29))
  (bind _coll_attack (Variables|Default|GetColl_Attack))
  (Networking|SwitchHasAuthority
    (:Authority
      (if (Variables|Default|GetbAttack)
        (bind _aschar_game (Utilities|Casting|CastToChar_Game OtherActor))
        (if (!= _aschar_game (Variables|Default|GetOwningPlayer))
          (Variables|Default|SetbAttack false)
          (Collision|SetCollisionEnabled _coll_attack "NoCollision")
          (Utilities|FlowControl|Delay 1.0)
          (Game|Damage|ApplyDamage _aschar_game (Variables|Default|GetDamage) 0 0)
          (Utilities|FlowControl|Delay 1.0)
          (Collision|SetCollisionEnabled _coll_attack "QueryAndPhysics"))))))

(fn ConstructionScript
  (|CallParentFunction))