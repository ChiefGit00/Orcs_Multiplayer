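; GS_Lobby is the lobby game state that holds the Players list.
; On BeginPlay, the authority copies MaxPlayers from GM_Lobby into NumberOfPlayers and uses it as the loop bound to fill Players with blank placeholder entries.
; GetPlayerInfo, despite its name, appends a new entry with the given player name and a different enum state, leaving the placeholders untouched.
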(event EventBeginPlay
  (Networking|SwitchHasAuthority
    (:Authority
      (bind _asgm_lobby (Utilities|Casting|CastToGM_Lobby (Game|GetGameMode)))
      (bind _output_get (Variables|Default|SetNumberOfPlayers (Variables|/Game/Blueprints/Gameplay/GM_Lobby.GM_Lobby_C|GetMaxPlayers _asgm_lobby)))
      (for _index (range 0 _output_get)
        (Utilities|Array|Add (Variables|Default|GetPlayers) (Utilities|Struct|MakeF_PlayerInfo "" "" "NewEnumerator2"))))))

(fn ConstructionScript)

(fn GetPlayerInfo
  (params (PlayerName :type String))
  (Utilities|Array|Add (Variables|Default|GetPlayers) (Utilities|Struct|MakeF_PlayerInfo PlayerName "" "NewEnumerator0")))