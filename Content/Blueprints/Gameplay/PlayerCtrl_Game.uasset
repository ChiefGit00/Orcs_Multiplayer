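; Player controller for a networked match game that tracks the player's replicated lives and owns the local gameplay HUD.
; Death decrements Life, updates the HUD, then after a short delay asks GM_Game for a game over or match over.
; Match-finish events reset the character, timer and BP_Shrine actors.
; At game end it disables input and shows a winner or loser screen based on remaining lives.
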(event Custom|Reset
  (Default|Reset (Variables|Default|GetPlayerChar)))

(event Custom|Death
  ;[1 1 1] Death
  (bind _result (Math|Integer|DecrementInt (Variables|Default|GetLife))
    (:%20%20
      (if (Pawn|IsLocalController)
        (Default|SetLife (Variables|Default|GetHUD) (Variables|Default|GetLife)))
      (Utilities|FlowControl|Delay 1.5)
      (bind _asgm_game (Utilities|Casting|CastToGM_Game (Game|GetGameMode)))
      (if (== _result 0)
        (Default|GameOver _asgm_game)
        (else
          (Default|MatchOver _asgm_game))))))

(event Custom|FinishHUD
  (params (InText :type Text))
  ;[1 1 1] Game Over
  (if (Pawn|IsLocalController)
    (Viewport|RemoveAllWidgets)
    (bind _returnvalue (UserInterface|CreateWidget "/Game/UI/WB_MatchFinish.WB_MatchFinish_C"))
    (Default|Result _returnvalue InText)
    (UserInterface|Viewport|AddtoViewport _returnvalue 0)
    (Variables|Default|SetbShowMouseCursor true)))

(event Custom|OC_MatchFinish
  ;[1 1 1] Match FInish
  (Variables|/Game/Blueprints/Actors/PlayerChars/Char_Game.Char_Game_C|SetTimer (Variables|Default|GetPlayerChar) 0)
  (Default|CallUpdateTimerHUD)
  (bind _outactors (Actor|GetAllActorsOfClass "/Game/Blueprints/Actors/BP_Shrine.BP_Shrine_C"))
  (for _array_element _outactors
    (Default|ResetShrine _array_element)))

(event Custom|S_MatchFinish
  ;[1 1 1] Match FInish
  (Default|Reset (Variables|Default|GetPlayerChar))
  (CallFunction|OCMatchFinish))

(event Custom|OC_GameFinishHUD
  ;[1 1 1] Game Over
  (Input|DisableInput (Pawn|GetControlledPawn) 0)
  (if (> (Variables|Default|GetLife) 0)
    (CallFunction|FinishHUD "Winner!!")
    (else
      (CallFunction|FinishHUD "Loser :("))))

(event EventBeginPlay
  (if (Pawn|IsLocalController)
    (bind _returnvalue (UserInterface|CreateWidget "/Game/UI/WB_HUD_Gameplay.WB_HUD_Gameplay_C"))
    (bind _output_get (Variables|Default|SetHUD _returnvalue))
    (UserInterface|Viewport|AddtoViewport _output_get 0)))

(event EventPossess
  (params (PossessedPawn :type Pawn%20Object%20Reference))
  (bind _aschar_game (Utilities|Casting|CastToChar_Game PossessedPawn))
  (Variables|Default|SetPlayerChar _aschar_game))

(fn ConstructionScript)

(fn OnRepLife
  (if (Pawn|IsLocalController)
    (Default|SetLife (Variables|Default|GetHUD) (Variables|Default|GetLife))))