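; GM_Game is the game mode that runs player spawning, the start countdown and match flow for a multiplayer game.
; BeginPlay gathers PlayerStarts and seeds GS_Game, then a short looping timer counts down before setting characters to Walking.
; PlayerJoin spawns, initializes and possesses each character from a DT_CharDataGame row.
; MatchOver notifies controllers, calls shrine recharge and respawns players as base Char_Game, while GameOver triggers each controller's finish HUD.
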(event Custom|MatchOver
  ;[1 1 1] Match Over
  (for _array_element (Variables|Default|GetPlayerCtrls)
    (Default|SMatchFinish _array_element))
  (bind _outactors (Actor|GetAllActorsOfClass "/Game/Blueprints/Actors/BP_Shrine.BP_Shrine_C"))
  (for _array_element_2 _outactors
    (Default|SAShrineRecharge _array_element_2))
  (bind _outactors_2 (Actor|GetAllActorsOfClass "/Game/Blueprints/Actors/PlayerChars/Game/Char_Game.Char_Game_C"))
  (for _array_element_3 _outactors_2
    (Actor|DestroyActor _array_element_3))
  (for (_array_element_4 _array_index) (Variables|Default|GetPlayerCtrls)
    (bind _returnvalue (Game|SpawnActorfromClass "/Game/Blueprints/Actors/PlayerChars/Game/Char_Game.Char_Game_C" (Math|Transform|MakeTransform (Transformation|GetActorLocation (Utilities|Array|Get(acopy) (Variables|Default|GetPlayerStarts) _array_index)) "0, 0, 0" "1,1,1") "Undefined" 0 0))
    (Pawn|Possess _array_element_4 _returnvalue)))

(event Custom|GameOver
  ;[1 1 1] Match Over
  ;;[1 1 1] Game Over
  (for _array_element (Variables|Default|GetPlayerCtrls)
    (Default|OCGameFinishHUD _array_element)))

(event Custom|PlayerJoin
  (params (PlayerChar :type Player%20Ctrl%20Game%20Object%20Reference) (CharCharRow :type Name) (Name :type String))
  ;[1 1 1] PlayerJoin
  (bind _returnvalue (Utilities|Array|Add (Variables|Default|GetPlayerCtrls) PlayerChar))
  (bind _asgs_game (Utilities|Casting|CastToGS_Game (Game|GetGameState)))
  (Default|AddPlayer _asgs_game Name)
  (bind _returnvalue_2 (Utilities|GetDataTableRow "/Game/Data/DT_CharDataGame.DT_CharDataGame" CharCharRow)
    (:then
      (bind _returnvalue_3 (Game|SpawnActorfromClass (.charclass _returnvalue_2) (Math|Transform|MakeTransform (Transformation|GetActorLocation (Utilities|Array|Get(acopy) (Variables|Default|GetPlayerStarts) _returnvalue)) "0, 0, 0" "1,1,1") "Undefined" 0 0))
      (bind _aschar_game (Utilities|Casting|CastToChar_Game _returnvalue_3))
      (Default|Init _aschar_game (.maxhealth _returnvalue_2) (.maxspeed _returnvalue_2) (.strength _returnvalue_2))
      (Pawn|Possess PlayerChar _aschar_game)
      (for _array_element (Variables|Default|GetPlayerCtrls)
        (Default|UpdatePlayerData _array_element)))))

(event Custom|CountDown
  (bind _gs_game (Variables|Default|GetGS_Game))
  (bind _output_get (Variables|/Game/Blueprints/Gameplay/GS_Game.GS_Game_C|SetTime _gs_game (- (Variables|/Game/Blueprints/Gameplay/GS_Game.GS_Game_C|GetTime _gs_game) 1)))
  (if (== _output_get 0)
    (Utilities|Time|ClearandInvalidateTimerbyHandle (stale EventBeginPlay _returnvalue))
    (bind _outactors (Actor|GetAllActorsOfClass "/Game/Blueprints/Actors/PlayerChars/Game/Char_Game.Char_Game_C"))
    (for _array_element _outactors
      (Pawn|Components|CharacterMovement|SetMovementMode (Variables|/Script/Engine.Character|GetCharacterMovement _array_element) "MOVE_Walking" 0))))

(event EventBeginPlay
  ;[1 1 1] BeginPlay (get PlayerStarts)
  (bind _outactors (Actor|GetAllActorsOfClass "/Script/Engine.PlayerStart"))
  (Variables|Default|SetPlayerStarts _outactors)
  (bind _asbp_game_instance (Utilities|Casting|CastToBP_GameInstance (Game|GetGameInstance)))
  (bind _asgs_game (Utilities|Casting|CastToGS_Game (Game|GetGameState)))
  (bind _output_get (Variables|Default|SetGS_Game _asgs_game))
  (Variables|/Game/Blueprints/Gameplay/GS_Game.GS_Game_C|SetTime _output_get 3)
  (Variables|/Game/Blueprints/Gameplay/GS_Game.GS_Game_C|SetNoOfPlayers _output_get (Variables|/Game/Blueprints/Gameplay/BP_GameInstance.BP_GameInstance_C|GetNoOfPlayers _asbp_game_instance))
  (bind _returnvalue (Utilities|Time|SetTimerbyEvent (delegate Custom|CountDown) 1.0 true)))

(fn ConstructionScript)