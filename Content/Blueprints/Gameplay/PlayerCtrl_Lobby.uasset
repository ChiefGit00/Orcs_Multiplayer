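; Lobby player controller that runs character selection and reports each player's choice to the game mode.
; On local BeginPlay it opens the selection widget and cycles DT_CharData rows with wraparound, updating stats and respawning a preview actor.
; Confirming swaps to game-only input with a lobby HUD, then S_CharSelected passes a class, hardcoded by row index, to GM_Lobby.Ready.
; UpdateHUD relays player counts to the local HUD through OC_UpdateLobbyHUD.
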(event Custom|SpawnChar
  (params (Class :type Actor%20Class%20Reference))
  ;[1 1 1] Spawn Charactor for selction
  (Utilities|IsValid (Variables|Default|GetCharActor)
    (:Is%20Valid
      (Actor|DestroyActor (Variables|Default|GetCharActor)))
    (:Is%20Not%20Valid
      _))
  (bind _returnvalue (Game|SpawnActorfromClass Class (Math|Transform|MakeTransform "0.000000,0.000000,500.000000" "0,180.000000, 0" "1,1,1") "AlwaysSpawn" 0 0))
  (Variables|Default|SetCharActor _returnvalue))

(event Custom|OC_UpdateLobbyHUD
  (params (InputPin :type Integer))
  ;[1 1 1] Lobby HUD Update
  (if (Pawn|IsLocalController)
    (Utilities|PlayerCountHUD)
    (Default|SetPlayerJoinedCount (Variables|Default|GetWB_LobbyHUD) InputPin)))

(event Custom|UpdateHUD
  (params (NoOfPlayers :type Integer))
  ;[1 1 1] Lobby HUD Update
  (CallFunction|OCUpdateLobbyHUD NoOfPlayers))

(event Custom|CharSelected
  (Utilities|PlayerCountHUD)
  (bind _charclass (CallFunction|GetCharClass))
  (CallFunction|SCharSelected _charclass))

(event Custom|S_CharSelected
  (params (CharClass :type Actor%20Class%20Reference))
  (bind _asgm_lobby (Utilities|Casting|CastToGM_Lobby (Game|GetGameMode)))
  (Default|Ready _asgm_lobby CharClass self))

(event EventBeginPlay
  ;[1 1 1] BeginPlay
  (if (Pawn|IsLocalController)
    (bind _returnvalue (UserInterface|CreateWidget "/Game/UI/WB_PlayerSelection.WB_PlayerSelection_C"))
    (bind _output_get (Variables|Default|SetHUD_Select _returnvalue))
    (UserInterface|Viewport|AddtoViewport _output_get 0)
    (Variables|Default|SetbShowMouseCursor true)
    (bind _outrownames (DataTable|GetDataTableRowNames "/Game/Data/DT_CharData.DT_CharData"))
    (bind _output_get_2 (Variables|Default|SetCharDT_Rows _outrownames))
    (Variables|Default|SetCharDT_Length (Utilities|Array|Length _output_get_2))
    (CallFunction|NextChar)))

(fn ConstructionScript)

(fn NextChar
  (params (Step :type Integer))
  (bind _output_get (Variables|Default|SetCurrentRow (+ Step (Variables|Default|GetCurrentRow))))
  (if (< _output_get (Variables|Default|GetCharDT_Length))
    (if (not (< (Variables|Default|GetCurrentRow) 0))
      _
      (else
        (Variables|Default|SetCurrentRow (- (Variables|Default|GetCharDT_Length) 1))))
    (else
      (Variables|Default|SetCurrentRow 0)))
  (bind _returnvalue (Utilities|GetDataTableRow "/Game/Data/DT_CharData.DT_CharData" (Utilities|Array|Get(acopy) (Variables|Default|GetCharDT_Rows) (Variables|Default|GetCurrentRow)))
    (:then
      (Default|SetData (Variables|/Game/UI/WB_PlayerSelection.WB_PlayerSelection_C|GetWB_PlayCharData (Variables|Default|GetHUD_Select)) (.charactername _returnvalue) (.maxhealth _returnvalue) (.maxspeed _returnvalue))
      (CallFunction|SpawnChar (.sk_mesh _returnvalue)))))

(fn GetCharClass
  (switch int (Variables|Default|GetCurrentRow)
    (:0
      (return "/Game/Blueprints/Actors/PlayerChars/Lobby/Char_Lobby_Orc01.Char_Lobby_Orc01_C"))
    (:1
      (return "/Game/Blueprints/Actors/PlayerChars/Lobby/Char_Lobby_Orc02.Char_Lobby_Orc02_C"))
    (:2
      (return "/Game/Blueprints/Actors/PlayerChars/Lobby/Char_Lobby_Orc03.Char_Lobby_Orc03_C"))
    (:3
      (return "/Game/Blueprints/Actors/PlayerChars/Lobby/Char_Lobby_Orc04.Char_Lobby_Orc04_C"))
    (:4
      (return "/Game/Blueprints/Actors/PlayerChars/Lobby/Char_Lobby_Orc05.Char_Lobby_Orc05_C"))
    (:5
      (return "/Game/Blueprints/Actors/PlayerChars/Lobby/Char_Lobby_Orc07.Char_Lobby_Orc07_C"))))