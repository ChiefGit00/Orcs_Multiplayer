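; Game state that tracks each player's name, life, kills and alive flag for a round-based elimination match.
; Health updates apply the delta, mark that player dead and report whether one or none remain; Reset revives everyone.
; Winner reports whether any player has reached the kill target.
; Replicated Time's OnRep passes the countdown to the local PlayerCtrl_Game.
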(fn ConstructionScript)

(fn InitPlayers
  (params (NoOfPlayers :type Integer)))

(fn SetPlayerName
  (params (Index :type Integer) (Name :type String))
  (|SetBy-RefVar (.playername (Utilities|Array|Get(acopy) (Variables|Default|GetPlayersData) Index)) Name))

(fn AddPlayer
  (params (PlayerName :type String))
  (Utilities|Array|Add (Variables|Default|GetPlayersData) (Utilities|Struct|MakeF_PlayerData PlayerName 3 0 true)))

(fn OnRepTime
  (bind _asplayer_ctrl_game (Utilities|Casting|CastToPlayerCtrl_Game (Game|GetPlayerController 0)))
  (Default|CountDown _asplayer_ctrl_game (Variables|Default|GetTime)))

(fn UpdatePlayerHealth
  (params (Index :type Integer) (LifeDelta :type Integer))
  (bind _playersdata (Variables|Default|GetPlayersData))
  (bind _output (Utilities|Array|Get(acopy) _playersdata Index))
  (|SetBy-RefVar (.life _output) (+ LifeDelta (.life _output)))
  (|SetBy-RefVar (.alive _output) false)
  (for _array_element (Variables|Default|GetPlayersData)
    (if (.alive _array_element)
      (Math|Integer|IncrementInt (LocalVariables|GetAliveCount))))
  (if (<= (LocalVariables|GetAliveCount) 1)
    (return true)
    (else
      (return false))))

(fn Reset
  (for _array_element (Variables|Default|GetPlayersData)
    (|SetBy-RefVar (.alive _array_element) true)))

(fn UpdateKill
  (params (Index :type Integer))
  (bind _playersdata (Variables|Default|GetPlayersData))
  (bind _output (Utilities|Array|Get(acopy) _playersdata Index))
  (|SetBy-RefVar (.kills _output) (+ (.kills _output) 1)))

(fn Winner
  (bind _array_element (Utilities|Array|ForEachLoopwithBreak (Variables|Default|GetPlayersData) :!label _label)
    (:LoopBody
      (if (>= (.kills _array_element) 3)
        (LocalVariables|SetbWinner true)
        (goto _label Break)))
    (:Completed
      (return (LocalVariables|GetbWinner)))))